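; Dirt plot actor that holds planted flowers, vegetables and other plants in slots tracked by the FlowersPlanted array.
; Each plant type has its own near-identical Plant function that finds the first invalid slot and spawns that class at the Dirtmesh socket named "attach_0" plus the index.
; The spawned plant receives this actor and its slot index.
; AddFlower writes a given plant into a slot, as the Plant functions do not fill the array themselves.
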(fn ConstructionScript)

(fn PlantADaisy
  (bind _self self)
  (Development|PrintString "planted")
  (bind (_array_element _array_index) (Utilities|Array|ForEachLoopwithBreak (Variables|Default|GetFlowersPlanted) :!label _label)
    (:LoopBody
      (if (not (Utilities|IsValid _array_element))
        (Game|SpawnActorfromClass "/Game/Blueprints/Daisyy.Daisyy_C" (Transformation|GetSocketTransform (Variables|Default|GetDirtmesh) (Utilities|String|StringToName (Utilities|String|Append (Utilities|String|MakeLiteralString "attach_0") (Utilities|String|ToString(Integer) _array_index))) "RTS_World") "AlwaysSpawn" "MultiplyWithRoot" _self _self _array_index 0 0)
        (goto _label Break)))))

(fn AddFlower
  (params (Index :type Integer) (Flower :type Flower%20Actor%20Object%20Reference))
  (Utilities|Array|SetArrayElem (Variables|Default|GetFlowersPlanted) Index Flower))

(fn PlantATomato
  (bind _self self)
  (Development|PrintString "planted")
  (bind (_array_element _array_index) (Utilities|Array|ForEachLoopwithBreak (Variables|Default|GetFlowersPlanted) :!label _label)
    (:LoopBody
      (if (not (Utilities|IsValid _array_element))
        (Game|SpawnActorfromClass "/Game/Blueprints/Tomatoo.Tomatoo_C" (Transformation|GetSocketTransform (Variables|Default|GetDirtmesh) (Utilities|String|StringToName (Utilities|String|Append (Utilities|String|MakeLiteralString "attach_0") (Utilities|String|ToString(Integer) _array_index))) "RTS_World") "AlwaysSpawn" "MultiplyWithRoot" _self _self _array_index 0 0)
        (goto _label Break)))))

(fn PlantABasil
  (bind _self self)
  (Development|PrintString "planted")
  (bind (_array_element _array_index) (Utilities|Array|ForEachLoopwithBreak (Variables|Default|GetFlowersPlanted) :!label _label)
    (:LoopBody
      (if (not (Utilities|IsValid _array_element))
        (Game|SpawnActorfromClass "/Game/Blueprints/Basill.Basill_C" (Transformation|GetSocketTransform (Variables|Default|GetDirtmesh) (Utilities|String|StringToName (Utilities|String|Append (Utilities|String|MakeLiteralString "attach_0") (Utilities|String|ToString(Integer) _array_index))) "RTS_World") "AlwaysSpawn" "MultiplyWithRoot" _self _self _array_index 0 0)
        (goto _label Break)))))

(fn PlantAPumpkin
  (bind _self self)
  (Development|PrintString "planted")
  (bind (_array_element _array_index) (Utilities|Array|ForEachLoopwithBreak (Variables|Default|GetFlowersPlanted) :!label _label)
    (:LoopBody
      (if (not (Utilities|IsValid _array_element))
        (Game|SpawnActorfromClass "/Game/Blueprints/Pumpkinn.Pumpkinn_C" (Transformation|GetSocketTransform (Variables|Default|GetDirtmesh) (Utilities|String|StringToName (Utilities|String|Append (Utilities|String|MakeLiteralString "attach_0") (Utilities|String|ToString(Integer) _array_index))) "RTS_World") "AlwaysSpawn" "MultiplyWithRoot" _self _self _array_index 0 0)
        (goto _label Break)))))

(fn PlantACalendula
  (bind _self self)
  (Development|PrintString "planted")
  (bind (_array_element _array_index) (Utilities|Array|ForEachLoopwithBreak (Variables|Default|GetFlowersPlanted) :!label _label)
    (:LoopBody
      (if (not (Utilities|IsValid _array_element))
        (Game|SpawnActorfromClass "/Game/Blueprints/Calendulaa.Calendulaa_C" (Transformation|GetSocketTransform (Variables|Default|GetDirtmesh) (Utilities|String|StringToName (Utilities|String|Append (Utilities|String|MakeLiteralString "attach_0") (Utilities|String|ToString(Integer) _array_index))) "RTS_World") "AlwaysSpawn" "MultiplyWithRoot" _self _self _array_index 0 0)
        (goto _label Break)))))

(fn PlantACarrot
  (bind _self self)
  (Development|PrintString "planted")
  (bind (_array_element _array_index) (Utilities|Array|ForEachLoopwithBreak (Variables|Default|GetFlowersPlanted) :!label _label)
    (:LoopBody
      (if (not (Utilities|IsValid _array_element))
        (Game|SpawnActorfromClass "/Game/Blueprints/Carrott.Carrott_C" (Transformation|GetSocketTransform (Variables|Default|GetDirtmesh) (Utilities|String|StringToName (Utilities|String|Append (Utilities|String|MakeLiteralString "attach_0") (Utilities|String|ToString(Integer) _array_index))) "RTS_World") "AlwaysSpawn" "MultiplyWithRoot" _self _self _array_index 0 0)
        (goto _label Break)))))

(fn PlantADaffadil
  (bind _self self)
  (Development|PrintString "planted")
  (bind (_array_element _array_index) (Utilities|Array|ForEachLoopwithBreak (Variables|Default|GetFlowersPlanted) :!label _label)
    (:LoopBody
      (if (not (Utilities|IsValid _array_element))
        (Game|SpawnActorfromClass "/Game/Blueprints/Daffadill.Daffadill_C" (Transformation|GetSocketTransform (Variables|Default|GetDirtmesh) (Utilities|String|StringToName (Utilities|String|Append (Utilities|String|MakeLiteralString "attach_0") (Utilities|String|ToString(Integer) _array_index))) "RTS_World") "AlwaysSpawn" "MultiplyWithRoot" _self _self _array_index 0 0)
        (goto _label Break)))))

(fn PlantALavender
  (bind _self self)
  (Development|PrintString "planted")
  (bind (_array_element _array_index) (Utilities|Array|ForEachLoopwithBreak (Variables|Default|GetFlowersPlanted) :!label _label)
    (:LoopBody
      (if (not (Utilities|IsValid _array_element))
        (Game|SpawnActorfromClass "/Game/Blueprints/Lavenderr.Lavenderr_C" (Transformation|GetSocketTransform (Variables|Default|GetDirtmesh) (Utilities|String|StringToName (Utilities|String|Append (Utilities|String|MakeLiteralString "attach_0") (Utilities|String|ToString(Integer) _array_index))) "RTS_World") "AlwaysSpawn" "MultiplyWithRoot" _self _self _array_index 0 0)
        (goto _label Break)))))

(fn PlantALettuce
  (bind _self self)
  (Development|PrintString "planted")
  (bind (_array_element _array_index) (Utilities|Array|ForEachLoopwithBreak (Variables|Default|GetFlowersPlanted) :!label _label)
    (:LoopBody
      (if (not (Utilities|IsValid _array_element))
        (Game|SpawnActorfromClass "/Game/Blueprints/Lettucee.Lettucee_C" (Transformation|GetSocketTransform (Variables|Default|GetDirtmesh) (Utilities|String|StringToName (Utilities|String|Append (Utilities|String|MakeLiteralString "attach_0") (Utilities|String|ToString(Integer) _array_index))) "RTS_World") "AlwaysSpawn" "MultiplyWithRoot" _self _self _array_index 0 0)
        (goto _label Break)))))

(fn PlantALilyOftheValley
  (bind _self self)
  (Development|PrintString "planted")
  (bind (_array_element _array_index) (Utilities|Array|ForEachLoopwithBreak (Variables|Default|GetFlowersPlanted) :!label _label)
    (:LoopBody
      (if (not (Utilities|IsValid _array_element))
        (Game|SpawnActorfromClass "/Game/Blueprints/LilyOfTheValleyyy.LilyOfTheValleyyy_C" (Transformation|GetSocketTransform (Variables|Default|GetDirtmesh) (Utilities|String|StringToName (Utilities|String|Append (Utilities|String|MakeLiteralString "attach_0") (Utilities|String|ToString(Integer) _array_index))) "RTS_World") "AlwaysSpawn" "MultiplyWithRoot" _self _self _array_index 0 0)
        (goto _label Break)))))

(fn PlantALily
  (bind _self self)
  (Development|PrintString "planted")
  (bind (_array_element _array_index) (Utilities|Array|ForEachLoopwithBreak (Variables|Default|GetFlowersPlanted) :!label _label)
    (:LoopBody
      (if (not (Utilities|IsValid _array_element))
        (Game|SpawnActorfromClass "/Game/Blueprints/Lilyy.Lilyy_C" (Transformation|GetSocketTransform (Variables|Default|GetDirtmesh) (Utilities|String|StringToName (Utilities|String|Append (Utilities|String|MakeLiteralString "attach_0") (Utilities|String|ToString(Integer) _array_index))) "RTS_World") "AlwaysSpawn" "MultiplyWithRoot" _self _self _array_index 0 0)
        (goto _label Break)))))

(fn PlantAPeriwinkle
  (bind _self self)
  (Development|PrintString "planted")
  (bind (_array_element _array_index) (Utilities|Array|ForEachLoopwithBreak (Variables|Default|GetFlowersPlanted) :!label _label)
    (:LoopBody
      (if (not (Utilities|IsValid _array_element))
        (Game|SpawnActorfromClass "/Game/Blueprints/Periwinklee.Periwinklee_C" (Transformation|GetSocketTransform (Variables|Default|GetDirtmesh) (Utilities|String|StringToName (Utilities|String|Append (Utilities|String|MakeLiteralString "attach_0") (Utilities|String|ToString(Integer) _array_index))) "RTS_World") "AlwaysSpawn" "MultiplyWithRoot" _self _self _array_index 0 0)
        (goto _label Break)))))

(fn PlantARadish
  (bind _self self)
  (Development|PrintString "planted")
  (bind (_array_element _array_index) (Utilities|Array|ForEachLoopwithBreak (Variables|Default|GetFlowersPlanted) :!label _label)
    (:LoopBody
      (if (not (Utilities|IsValid _array_element))
        (Game|SpawnActorfromClass "/Game/Blueprints/Radishh.Radishh_C" (Transformation|GetSocketTransform (Variables|Default|GetDirtmesh) (Utilities|String|StringToName (Utilities|String|Append (Utilities|String|MakeLiteralString "attach_0") (Utilities|String|ToString(Integer) _array_index))) "RTS_World") "AlwaysSpawn" "MultiplyWithRoot" _self _self _array_index 0 0)
        (goto _label Break)))))

(fn PlantASunflower
  (bind _self self)
  (Development|PrintString "planted")
  (bind (_array_element _array_index) (Utilities|Array|ForEachLoopwithBreak (Variables|Default|GetFlowersPlanted) :!label _label)
    (:LoopBody
      (if (not (Utilities|IsValid _array_element))
        (Game|SpawnActorfromClass "/Game/Blueprints/Sunflowerr.Sunflowerr_C" (Transformation|GetSocketTransform (Variables|Default|GetDirtmesh) (Utilities|String|StringToName (Utilities|String|Append (Utilities|String|MakeLiteralString "attach_0") (Utilities|String|ToString(Integer) _array_index))) "RTS_World") "AlwaysSpawn" "MultiplyWithRoot" _self _self _array_index 0 0)
        (goto _label Break)))))

(fn PlantATulip
  (bind _self self)
  (Development|PrintString "planted")
  (bind (_array_element _array_index) (Utilities|Array|ForEachLoopwithBreak (Variables|Default|GetFlowersPlanted) :!label _label)
    (:LoopBody
      (if (not (Utilities|IsValid _array_element))
        (Game|SpawnActorfromClass "/Game/Blueprints/Tulipp.Tulipp_C" (Transformation|GetSocketTransform (Variables|Default|GetDirtmesh) (Utilities|String|StringToName (Utilities|String|Append (Utilities|String|MakeLiteralString "attach_0") (Utilities|String|ToString(Integer) _array_index))) "RTS_World") "AlwaysSpawn" "MultiplyWithRoot" _self _self _array_index 0 0)
        (goto _label Break)))))

(fn PlantARose
  (bind _self self)
  (Development|PrintString "planted")
  (bind (_array_element _array_index) (Utilities|Array|ForEachLoopwithBreak (Variables|Default|GetFlowersPlanted) :!label _label)
    (:LoopBody
      (if (not (Utilities|IsValid _array_element))
        (Game|SpawnActorfromClass "/Game/Blueprints/Rosee.Rosee_C" (Transformation|GetSocketTransform (Variables|Default|GetDirtmesh) (Utilities|String|StringToName (Utilities|String|Append (Utilities|String|MakeLiteralString "attach_0") (Utilities|String|ToString(Integer) _array_index))) "RTS_World") "AlwaysSpawn" "MultiplyWithRoot" _self _self _array_index 0 0)
        (goto _label Break)))))

(fn PlantAVenusFlytrap
  (bind _self self)
  (Development|PrintString "planted")
  (bind (_array_element _array_index) (Utilities|Array|ForEachLoopwithBreak (Variables|Default|GetFlowersPlanted) :!label _label)
    (:LoopBody
      (if (not (Utilities|IsValid _array_element))
        (Game|SpawnActorfromClass "/Game/Blueprints/VenusFlyy.VenusFlyy_C" (Transformation|GetSocketTransform (Variables|Default|GetDirtmesh) (Utilities|String|StringToName (Utilities|String|Append (Utilities|String|MakeLiteralString "attach_0") (Utilities|String|ToString(Integer) _array_index))) "RTS_World") "AlwaysSpawn" "MultiplyWithRoot" _self _self _array_index 0 0)
        (goto _label Break)))))

(fn PlantAOrchid
  (bind _self self)
  (Development|PrintString "planted")
  (bind (_array_element _array_index) (Utilities|Array|ForEachLoopwithBreak (Variables|Default|GetFlowersPlanted) :!label _label)
    (:LoopBody
      (if (not (Utilities|IsValid _array_element))
        (Game|SpawnActorfromClass "/Game/Blueprints/Orchidd.Orchidd_C" (Transformation|GetSocketTransform (Variables|Default|GetDirtmesh) (Utilities|String|StringToName (Utilities|String|Append (Utilities|String|MakeLiteralString "attach_0") (Utilities|String|ToString(Integer) _array_index))) "RTS_World") "AlwaysSpawn" "MultiplyWithRoot" _self _self _array_index 0 0)
        (goto _label Break)))))

(fn PlantASucc
  (bind _self self)
  (Development|PrintString "planted")
  (bind (_array_element _array_index) (Utilities|Array|ForEachLoopwithBreak (Variables|Default|GetFlowersPlanted) :!label _label)
    (:LoopBody
      (if (not (Utilities|IsValid _array_element))
        (Game|SpawnActorfromClass "/Game/Blueprints/Succulentt.Succulentt_C" (Transformation|GetSocketTransform (Variables|Default|GetDirtmesh) (Utilities|String|StringToName (Utilities|String|Append (Utilities|String|MakeLiteralString "attach_0") (Utilities|String|ToString(Integer) _array_index))) "RTS_World") "AlwaysSpawn" "MultiplyWithRoot" _self _self _array_index 0 0)
        (goto _label Break)))))

(fn PlantAWatermelon
  (bind _self self)
  (Development|PrintString "planted")
  (bind (_array_element _array_index) (Utilities|Array|ForEachLoopwithBreak (Variables|Default|GetFlowersPlanted) :!label _label)
    (:LoopBody
      (if (not (Utilities|IsValid _array_element))
        (Game|SpawnActorfromClass "/Game/Blueprints/Watermelonn.Watermelonn_C" (Transformation|GetSocketTransform (Variables|Default|GetDirtmesh) (Utilities|String|StringToName (Utilities|String|Append (Utilities|String|MakeLiteralString "attach_0") (Utilities|String|ToString(Integer) _array_index))) "RTS_World") "AlwaysSpawn" "MultiplyWithRoot" _self _self _array_index 0 0)
        (goto _label Break)))))