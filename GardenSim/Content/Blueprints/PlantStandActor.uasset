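; PlantStandActor is a plant stand actor that positions flowers for sale on its mesh sockets.
; SellADaisyy scans PlantsSelling and, for each invalid entry, moves the given flower to the socket named "attach_0" plus that index.
; The loop has no break and never writes to the array, so the flower ends at the last empty slot.
; AddFlowerToSelling and the event graph are empty stubs.
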(event EventBeginPlay)

(event Collision|EventActorBeginOverlap
  (params (OtherActor :type Actor%20Object%20Reference)))

(event EventTick
  (params (DeltaSeconds :type Float%20%28single-precision%29)))

(fn ConstructionScript)

(fn SellADaisyy
  (params (Flower :type Flower%20Actor%20Object%20Reference))
  (bind (_array_element _array_index) (Utilities|Array|ForEachLoopwithBreak (Variables|Default|GetPlantsSelling))
    (:LoopBody
      (if (not (Utilities|IsValid _array_element))
        (Transformation|SetActorTransform Flower (Transformation|GetSocketTransform (Variables|Default|Getstandstaticm) (Utilities|String|StringToName (Utilities|String|Append (Utilities|String|MakeLiteralString "attach_0") (Utilities|String|ToString(Integer) _array_index))) "RTS_World"))))))

(fn AddFlowertoSelling)